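; BP_Bullet is a bullet actor that explodes on contact and destroys whatever actor its collision component overlaps.
; On overlap it spawns a half-scale explosion emitter at its location, then destroys the other actor and itself, with no type check.
; On a blocking hit it spawns the same effect and destroys only itself.
; An AI_Enemy cast that subtracts health and destroys at zero is left disconnected and never runs.
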(event `self.CollisionComp.OnComponentBeginOverlap`
  (params (OverlappedComponent :type "PrimitiveComponent Object Reference") (OtherActor :type "Actor Object Reference") (OtherComp :type "PrimitiveComponent Object Reference") (OtherBodyIndex :type Integer) (bFromSweep :type Boolean) (SweepResult :type "HitResult Structure (by ref)"))
  (`GameplayStatics.SpawnEmitterAtLocation` "/Game/StarterContent/Particles/P_Explosion.P_Explosion" (`self.K2_GetActorLocation`) (struct) (0.5 0.5 0.5))
  (`self.K2_DestroyActor` OtherActor)
  (`self.K2_DestroyActor`))

(event `self.CollisionComp.OnComponentHit`
  (params (HitComponent :type "PrimitiveComponent Object Reference") (OtherActor :type "Actor Object Reference") (OtherComp :type "PrimitiveComponent Object Reference") (NormalImpulse :type "Vector Structure") (Hit :type "HitResult Structure (by ref)"))
  (`GameplayStatics.SpawnEmitterAtLocation` "/Game/StarterContent/Particles/P_Explosion.P_Explosion" (`self.K2_GetActorLocation`) (struct) (0.5 0.5 0.5))
  (`self.K2_DestroyActor`))

(fn `UserConstructionScript`)