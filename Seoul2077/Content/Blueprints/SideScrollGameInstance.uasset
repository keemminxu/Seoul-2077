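; SideScrollGameInstance is a game instance Blueprint that manages the main gameplay HUD for a side-scrolling game.
; ShowGamePlayMainWidget lazily creates the GamePlayMain widget for the first player controller, caches it, then adds it to or removes it from the viewport.
; UpdateHeroHPBar sets the hero's HP progress bar from the current-to-max HP ratio.
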(fn `Show Game Play Main Widget`
  (params (`Is Show` :type Boolean))
  (bind _game_play_main_widget_ref (`self.Game Play Main Widget Ref`))
  (`/Engine/EditorBlueprintResources/StandardMacros.IsValid` (`self.Game Play Main Widget Ref`)
    (:`Is Valid`
      _)
    (:`Is Not Valid`
      (bind _returnvalue (`|CreateWidget` "/Game/Blueprints/GamePlayMain.GamePlayMain_C" (`GameplayStatics.GetPlayerController` 0)))
      (set `self.Game Play Main Widget Ref` _returnvalue)))
  (if `Is Show`
    (`UserWidget.AddToViewport` _game_play_main_widget_ref 0)
    (else
      (`Widget.RemoveFromParent` _game_play_main_widget_ref))))

(fn `Update Hero HPBar`
  (params (HP :type "Float (double-precision)") (`Max HP` :type "Float (double-precision)"))
  (`ProgressBar.SetPercent` (`self.Progress BarHP`) (/ HP `Max HP`)))