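; BP_AIFactory is an enemy spawner actor that creates BP_Gaurd actors at its own transform.
; On Tick it sets CurrentTime to zero, then calls CreateEnemy if that plus the frame delta exceeds CreateTime.
; Time never accumulates across frames, so spawning happens only when a single frame's delta exceeds CreateTime.
; CreateEnemy spawns the guard and zeroes CurrentTime again.
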(event `self.ReceiveTick`
  (params (DeltaSeconds :type "Float (single-precision)"))
  (set `self.CurrentTime` 0.0)
  (if (> (+ DeltaSeconds (`self.CurrentTime`)) (`self.CreateTime`))
    (`self.CreateEnemy`)))

(fn `CreateEnemy`
  (`|SpawnActorFromClass` "/Game/ai11/AI/BP_Gaurd.BP_Gaurd_C" (`self.GetTransform`) "Undefined" "OverrideRootScale" null null)
  (set `self.CurrentTime` 0.0))

(fn `UserConstructionScript`)