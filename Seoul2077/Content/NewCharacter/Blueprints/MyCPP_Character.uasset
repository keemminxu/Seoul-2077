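; Player character Blueprint that handles sprint input, camera boom zoom and sprint camera shake.
; Sprint input toggles IsSprinting and runs a timeline that lengthens the boom, but sets WalkingSpeed on press and SprintSpeed on release, apparently swapped.
; A SprintingCameraShake event, not called in this graph, starts or stops the shake by velocity.
; Its start branch requires the shaking flag to already be true.
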(event `Sprinting Camera Shake`
  (bind _returnvalue (`GameplayStatics.GetPlayerCameraManager` 0))
  (if (> (`KismetMathLibrary.VSize` (`MovementComponent.Velocity` (`self.CharacterMovement`))) (+ (`self.Walking Speed`) 50.0))
    (if (`self.Is Sprinting`)
      (if (`self.Sprinting Camera Shaking`)
        (bind _returnvalue_2 (`PlayerCameraManager.StartCameraShake` :`self` _returnvalue :`ShakeClass` "/Game/NewCharacter/Effects/Camera_Shakes/Sprinting_Cshake.Sprinting_Cshake_C" :`Scale` (`self.Sprinting Camera Shake Scale`)))
        (set `self.Sprinting Camera Shake instance` _returnvalue_2)
        (set `self.Sprinting Camera Shaking` true)))
    (elif (`self.Sprinting Camera Shaking`)
      (`PlayerCameraManager.StopCameraShake` _returnvalue (`self.Sprinting Camera Shake instance`) true)
      (set `self.Sprinting Camera Shaking` false))))

(event `InputAction|Sprinting`
  (params (Key :type "Key Structure"))
  (bind _charactermovement (`self.CharacterMovement`))
  (:`Pressed`
    (set `CharacterMovementComponent.MaxWalkSpeed` (`self.Walking Speed`) _charactermovement)
    (set `self.Is Sprinting` true)
    (bind (_direction _value) (`Timeline|Timeline_0` :!label _label)
      (:`Update`
        (set `SpringArmComponent.TargetArmLength` (`KismetMathLibrary.Lerp` 300.0 350.0 _value) (`self.CameraBoom`)))))
  (:`Released`
    (set `CharacterMovementComponent.MaxWalkSpeed` (`self.Sprint Speed`) _charactermovement)
    (set `self.Is Sprinting` false)
    (goto _label :!via `Reverse`)))

(fn `UserConstructionScript`)